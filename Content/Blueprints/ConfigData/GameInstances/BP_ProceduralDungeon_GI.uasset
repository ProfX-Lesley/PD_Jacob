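; Game instance Blueprint for procedural dungeon generation that sets up a seed and spawns the starting room.
; InitializeDungeonIF randomizes SeedStream and records its seed when LoadingSeed is zero, then spawns the room at StartRoomSpawnPoint.
; Applying a nonzero LoadingSeed to the stream is unreachable, and room choice always returns the first StartRoomClasses entry, leaving the seeded random pick unused.
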(event `/Game/Blueprints/Interfaces/BPI_ProceduralDungeon.InitializeDungeon_IF`
  (`self.ProcessSeedInput`)
  (`self.GenerateStarterRoom`))

(fn `GenerateStarterRoom`
  (`|SpawnActorFromClass` (`self.RandomizeStartRoom`) (`self.StartRoomSpawnPoint`) "Undefined" "MultiplyWithRoot" null null))

(fn `ProcessSeedInput`
  (bind _seedstream_initialseed (`KismetMathLibrary.BreakRandomStream` (`self.SeedStream`)))
  (if (== (`self.LoadingSeed`) 0)
    (`KismetMathLibrary.SeedRandomStream` (`self.SeedStream`))
    (set `self.LoadingSeed` _seedstream_initialseed)))

(fn `RandomizeStartRoom`
  (returns (StartRoomClass :type "/Game/Blueprints/Actors/DungeonRooms/BP_Room_Master Class Reference"))
  (return (`|GetArrayItem` (`self.StartRoomClasses`))))